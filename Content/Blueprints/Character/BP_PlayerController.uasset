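; Player controller that routes movement, look, free look and inventory input to BP_Player and BP_HUD.
; Stand, crouch and prone changes resolve through data-table transitions, with timed transitions blocking movement until a timer fires.
; Pose-keyed tables also drive pitch limits and camera height, both eased by timelines.
; Walk speed is cached by weapon, pose and move state, then chosen by whether acceleration falls within the forward arc.
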(event Custom|SetEnableMove
  ;[0.15 0.15 0.15 0.5] FSM Finite_State_Machine 유한 상태 머신.
  (Variables|Pose|SetbIsEnableMove true))

(event Custom|OnMovementStateChanged
  (params (bIsMovingNow :type Boolean))
  ;[0.15 0.15 0.15 0.5] 플레이어 Ref 저장
  (Camera|UpdateCameraHeight false))

(event EventBeginPlay
  ;[0.15 0.15 0.15 0.5] 플레이어 Ref 저장
  (bind _asbp_player (Utilities|Casting|CastToBP_Player (Game|GetPlayerCharacter 0)))
  (Utilities|IsValid _asbp_player
    (:Is%20Valid
      (Variables|Ref|SetBP_PlayerRef _asbp_player)
      (Camera|UpdatePitchLimits "NewEnumerator0")
      (EventDispatchers|BindEventtoOnMovementStateChange (Variables|Ref|GetBP_PlayerRef) (delegate Custom|OnMovementStateChanged))
      (CallFunction|SetCachedWalkSpeed)
      (bind _asbp_hud (Utilities|Casting|CastToBP_HUD (HUD|GetHUD)))
      (Utilities|IsValid _asbp_hud
        (:Is%20Valid
          (Variables|Ref|SetHUD_Ref _asbp_hud))))))

(event Input|ActionEvents|InputActionWalk
  (params (Key :type Key%20Structure :default "None"))
  (bind _bp_playerref (Variables|Ref|GetBP_PlayerRef))
  ;[0.15 0.15 0.15 0.5] Movement 상태 업데이트
  (:Pressed
    (Variables|/Game/Blueprints/Character/BP_Player.BP_Player_C|SetbIsWalkPressed _bp_playerref true)
    (Default|EvaluateMoveState (Variables|Ref|GetBP_PlayerRef) :!label _label)
    (CallFunction|SetCachedWalkSpeed))
  (:Released
    (Variables|/Game/Blueprints/Character/BP_Player.BP_Player_C|SetbIsWalkPressed _bp_playerref false)
    (goto _label)))

(event Input|ActionEvents|InputActionFreeLook
  (params (Key :type Key%20Structure :default "None"))
  (bind _bp_playerref (Variables|Ref|GetBP_PlayerRef))
  ;[0.15 0.15 0.15 0.5] FreeLook
  (:Pressed
    (Default|FreeLook _bp_playerref true))
  (:Released
    (Default|FreeLook _bp_playerref false)))

(event Input|ActionEvents|InputActionCrouch
  (params (Key :type Key%20Structure :default "None"))
  (bind _bp_playerref (Variables|Ref|GetBP_PlayerRef))
  (bind _currentposestate (Variables|/Game/Blueprints/Character/BP_Player.BP_Player_C|GetCurrentPoseState _bp_playerref))
  (bind _bisweaponequipped (Variables|/Game/Blueprints/Character/BP_Player.BP_Player_C|GetbIsWeaponEquipped _bp_playerref))
  (bind (_transitiontime _topose) (Pose|OnTransitionTimer "NewEnumerator1" _currentposestate _bisweaponequipped))
  ;[0.15 0.15 0.15 0.5] FSM Finite_State_Machine 유한 상태 머신.
  (:Pressed
    (Pose|UpdatePose _transitiontime _topose)
    (Camera|UpdatePitchLimits (Variables|/Game/Blueprints/Character/BP_Player.BP_Player_C|GetCurrentPoseState (Variables|Ref|GetBP_PlayerRef)))
    (Camera|UpdateCameraHeight false)
    (CallFunction|SetCachedWalkSpeed)))

(event Input|ActionEvents|InputActionProne
  (params (Key :type Key%20Structure :default "None"))
  (bind _bp_playerref (Variables|Ref|GetBP_PlayerRef))
  (bind _currentposestate (Variables|/Game/Blueprints/Character/BP_Player.BP_Player_C|GetCurrentPoseState _bp_playerref))
  (bind _bisweaponequipped (Variables|/Game/Blueprints/Character/BP_Player.BP_Player_C|GetbIsWeaponEquipped _bp_playerref))
  (bind (_transitiontime _topose) (Pose|OnTransitionTimer "NewEnumerator2" _currentposestate _bisweaponequipped))
  ;[0.15 0.15 0.15 0.5] FSM Finite_State_Machine 유한 상태 머신.
  (:Pressed
    (Pose|UpdatePose _transitiontime _topose)
    (Camera|UpdatePitchLimits (Variables|/Game/Blueprints/Character/BP_Player.BP_Player_C|GetCurrentPoseState (Variables|Ref|GetBP_PlayerRef)))
    (Camera|UpdateCameraHeight false)
    (CallFunction|SetCachedWalkSpeed)))

(event Input|ActionEvents|InputActionJump
  (params (Key :type Key%20Structure :default "None"))
  (bind _bp_playerref (Variables|Ref|GetBP_PlayerRef))
  (bind _bisweaponequipped (Variables|/Game/Blueprints/Character/BP_Player.BP_Player_C|GetbIsWeaponEquipped _bp_playerref))
  (bind _currentposestate (Variables|/Game/Blueprints/Character/BP_Player.BP_Player_C|GetCurrentPoseState _bp_playerref))
  (bind (_transitiontime _topose) (Pose|OnTransitionTimer "NewEnumerator0" _currentposestate _bisweaponequipped))
  ;[0.15 0.15 0.15 0.5] FSM Finite_State_Machine 유한 상태 머신.
  (:Pressed
    (if (Utilities|Enum|Equal(Enum) _currentposestate "NewEnumerator0")
      (Character|Jump (Variables|Ref|GetBP_PlayerRef))
      (else
        (Pose|UpdatePose _transitiontime _topose)
        (Camera|UpdatePitchLimits (Variables|/Game/Blueprints/Character/BP_Player.BP_Player_C|GetCurrentPoseState (Variables|Ref|GetBP_PlayerRef)))
        (Camera|UpdateCameraHeight false)
        (CallFunction|SetCachedWalkSpeed)))))

(event Input|ActionEvents|InputActionRun
  (params (Key :type Key%20Structure :default "None"))
  (bind _bp_playerref (Variables|Ref|GetBP_PlayerRef))
  ;[0.15 0.15 0.15 0.5] Movement 상태 업데이트
  (:Pressed
    (Variables|/Game/Blueprints/Character/BP_Player.BP_Player_C|SetbIsRunPresssed _bp_playerref true)
    (Default|EvaluateMoveState (Variables|Ref|GetBP_PlayerRef) :!label _label)
    (CallFunction|SetCachedWalkSpeed))
  (:Released
    (Variables|/Game/Blueprints/Character/BP_Player.BP_Player_C|SetbIsRunPresssed _bp_playerref false)
    (goto _label)))

(event Input|ActionEvents|InputActionInventory
  (params (Key :type Key%20Structure :default "None"))
  ;[0.15 0.15 0.15 0.5] 인벤토리 토글키
  (:Pressed
    (Default|ToggleInventoryUI (Variables|Ref|GetHUD_Ref))))

(event Input|AxisEvents|InputAxisTurn
  (params (AxisValue :type Float%20%28single-precision%29))
  ;[0.15 0.15 0.15 0.5] 마우스 input
  (if (not (Variables|Default|GetbShowMouseCursor))
    (Default|InputTurn (Variables|Ref|GetBP_PlayerRef) AxisValue)))

(event Input|AxisEvents|InputAxisLookUp
  (params (AxisValue :type Float%20%28single-precision%29))
  ;[0.15 0.15 0.15 0.5] 마우스 input
  (if (Camera|LimitPicthAngle AxisValue)
    (if (not (Variables|Default|GetbShowMouseCursor))
      (Default|InputLookUp (Variables|Ref|GetBP_PlayerRef) AxisValue))))

(event Input|AxisEvents|InputAxisMoveForward
  (params (AxisValue :type Float%20%28single-precision%29))
  ;[0.15 0.15 0.15 0.5] 키보드 input
  (if (Variables|Pose|GetbIsEnableMove)
    (CallFunction|UpdateWalkSpeed)
    (Default|Move (Variables|Ref|GetBP_PlayerRef) true AxisValue)))

(event Input|AxisEvents|InputAxisMoveRight
  (params (AxisValue :type Float%20%28single-precision%29))
  ;[0.15 0.15 0.15 0.5] 키보드 input
  (if (Variables|Pose|GetbIsEnableMove)
    (CallFunction|UpdateWalkSpeed)
    (Default|Move (Variables|Ref|GetBP_PlayerRef) false AxisValue)))

(event Custom|SetPitchRotation
  (params (CurrentRotation :type Rotator) (NextRotation :type Rotator))
  (bind _alpha (Timeline|SetPitchRotator PlayFromStart)
    (:Update
      (Pawn|SetControlRotation (Math|Rotator|Lerp(Rotator) CurrentRotation NextRotation _alpha)))))

(event Custom|ChangeCameraHeight
  (params (CurrentHeight :type Float%20%28double-precision%29) (TargetHeight :type Float%20%28double-precision%29))
  (bind _bp_playerref (Variables|Ref|GetBP_PlayerRef))
  (bind _springarm (Variables|/Game/Blueprints/Character/BP_Player.BP_Player_C|GetSpringArm _bp_playerref))
  (bind _alpha (Timeline|TL_ChangeCameraHeight PlayFromStart)
    (:Update
      (Variables|/Script/Engine.SpringArmComponent|SetSocketOffset _springarm (Math|Vector|MakeVector (.x (Variables|/Script/Engine.SpringArmComponent|GetSocketOffset _springarm)) (.y (Variables|/Script/Engine.SpringArmComponent|GetSocketOffset _springarm)) (Math|Float|Lerp CurrentHeight TargetHeight _alpha))))))

(fn ConstructionScript)

(fn TryGetPoseTransition
  (params (TargetPose :type E_PoseState%20Enum :default "NewEnumerator0") (FromPose :type E_PoseState%20Enum :default "NewEnumerator0"))
  (bind _returnvalue (Utilities|GetDataTableRow "/Game/Blueprints/Datas/DataTable/DT_PoseTransitions.DT_PoseTransitions" (Utilities|String|StringToName (Utilities|String|Append (Utilities|String|EnumtoString TargetPose) "_" (Utilities|String|EnumtoString FromPose))))
    (:then
      (return (.topose _returnvalue)))
    (:RowNotFound
      (Development|PrintString "못 찾음" true true "(R=1.000000,G=0.000000,B=0.000000,A=1.000000)" 999.0))))

(fn OnTransitionTimer
  (params (TargetPose :type E_PoseState%20Enum :default "NewEnumerator0") (FromPose :type E_PoseState%20Enum :default "NewEnumerator0") (bIsWeaponEquipped :type Boolean))
  (LocalVariables|SetReturnPose (Pose|TryGetPoseTransition TargetPose FromPose))
  (bind _returnvalue (Utilities|GetDataTableRow "/Game/Blueprints/Datas/DataTable/DT_ProneTime.DT_ProneTime" (Utilities|String|StringToName (Utilities|String|Append (Utilities|String|ToString(Boolean) bIsWeaponEquipped) "_" (Utilities|String|EnumtoString FromPose) "_" (Utilities|String|EnumtoString (LocalVariables|GetReturnPose)))))
    (:then
      _)
    (:RowNotFound
      _))
  (return (.sec _returnvalue) (LocalVariables|GetReturnPose)))

(fn UpdatePose
  (params (Wait%20Time :type Float%20%28double-precision%29) (ToPose :type E_PoseState%20Enum :default "NewEnumerator0"))
  (if (!= Wait%20Time 0.0)
    (Variables|Pose|SetbIsEnableMove false)
    (Utilities|Time|SetTimerbyEvent (EventDispatchers|CreateEvent :!event Custom|SetEnableMove) Wait%20Time)
    (Default|UpdatePoseState (Variables|Ref|GetBP_PlayerRef) ToPose)
    (else
      (Default|UpdatePoseState (Variables|Ref|GetBP_PlayerRef) ToPose))))

(fn UpdatePitchLimits
  (params (ToPose :type E_PoseState%20Enum :default "NewEnumerator0"))
  (bind _returnvalue (Pawn|GetControlRotation :!class /Script/Engine.Controller))
  (bind _returnvalue_2 (Pawn|GetControlRotation :!class /Script/Engine.Controller))
  (bind _returnvalue_3 (Pawn|GetControlRotation :!class /Script/Engine.Controller))
  (Utilities|FlowControl|Sequence
    (:then_0
      (bind _returnvalue_4 (Utilities|GetDataTableRow "/Game/Blueprints/Datas/DataTable/DT_PitchLimits.DT_PitchLimits" (Utilities|String|StringToName (Utilities|String|EnumtoString ToPose)))
        (:then
          (Variables|Camera|SetCachedTopLimit (.toplimit _returnvalue_4))
          (Variables|Camera|SetCachedBottomLimit (.bottomlimit _returnvalue_4)))))
    (:then_1
      (if (not (or (> (.pitch _returnvalue) (Variables|Camera|GetCachedBottomLimit)) (< (.pitch _returnvalue) (Variables|Camera|GetCachedTopLimit))))
        (if (< (Math|Float|Absolute(Float) (- (.pitch _returnvalue) (Variables|Camera|GetCachedTopLimit))) (Math|Float|Absolute(Float) (- (.pitch _returnvalue) (Variables|Camera|GetCachedBottomLimit))))
          (CallFunction|SetPitchRotation (Pawn|GetControlRotation :!class /Script/Engine.Controller) (Math|Rotator|MakeRotator (.roll _returnvalue_3) (Variables|Camera|GetCachedTopLimit) (.yaw _returnvalue_3)))
          (else
            (CallFunction|SetPitchRotation (Pawn|GetControlRotation :!class /Script/Engine.Controller) (Math|Rotator|MakeRotator (.roll _returnvalue_2) (Variables|Camera|GetCachedBottomLimit) (.yaw _returnvalue_2)))))))))

(fn LimitPicthAngle
  (params (Axis :type Float%20%28double-precision%29))
  (bind _returnvalue (Pawn|GetControlRotation :!class /Script/Engine.Controller))
  (bind _returnvalue_2 (Class|PlayerController|GetDeprecatedInputPitchScale))
  (bind _returnvalue_3 (* Axis _returnvalue_2))
  (bind _returnvalue_4 (+ (.pitch _returnvalue) _returnvalue_3))
  (return (or (> _returnvalue_4 (Variables|Camera|GetCachedBottomLimit)) (< _returnvalue_4 (Variables|Camera|GetCachedTopLimit)))))

(fn UpdateCameraHeight
  (params (IsMovingNow :type Boolean))
  (bind _bp_playerref (Variables|Ref|GetBP_PlayerRef))
  (bind _currentposestate (Variables|/Game/Blueprints/Character/BP_Player.BP_Player_C|GetCurrentPoseState _bp_playerref))
  (Utilities|FlowControl|Sequence
    (:then_0
      (LocalVariables|SetCurrentPose (Utilities|String|EnumtoString _currentposestate))
      (if (Utilities|Enum|NotEqual(Enum) _currentposestate "NewEnumerator1")
        ;[0.15 0.15 0.15 0.5] Stand 혹은 Prone일 때
        (LocalVariables|SetRowName (LocalVariables|GetCurrentPose))
        (else
          ;[0.15 0.15 0.15 0.5] Crouch 인데 움직이지 않을 때
          (LocalVariables|SetRowName (LocalVariables|GetCurrentPose))
          ;[0.15 0.15 0.15 0.5] Crouch 인데 움직이는 경우
          (if IsMovingNow
            (LocalVariables|SetRowName (Utilities|String|Append (LocalVariables|GetCurrentPose) "_" (Utilities|String|ToString(Boolean) (Variables|/Game/Blueprints/Character/BP_Player.BP_Player_C|GetbIsWeaponEquipped (Variables|Ref|GetBP_PlayerRef))) "_Move"))))))
    (:then_1
      ;[0.15 0.15 0.15 0.5] 무슨 상태인지 판별 후 카메라 위치 조정
      (bind _returnvalue (Utilities|GetDataTableRow "/Game/Blueprints/Datas/DataTable/DT_CameraHeight.DT_CameraHeight" (Utilities|String|StringToName (LocalVariables|GetRowName)))
        (:then
          (CallFunction|ChangeCameraHeight (.z (Variables|/Script/Engine.SpringArmComponent|GetSocketOffset (Variables|/Game/Blueprints/Character/BP_Player.BP_Player_C|GetSpringArm (Variables|Ref|GetBP_PlayerRef)))) (.height _returnvalue)))))))

(fn UpdateWalkSpeed
  (bind _cachedspeeddata (Variables|Default|GetCachedSpeedData))
  ;[0.15 0.15 0.15 0.5] 저장된 WalkSpeed를 적용하는 부분
  (Default|SetMaxWalkSpeed (Variables|Ref|GetBP_PlayerRef) (Math|Float|SelectFloat (.forwardspeed _cachedspeeddata) (.noneforwardspeed _cachedspeeddata) (CallFunction|IsAcceleratingForwardArc))))

(fn IsAcceleratingForwardArc
  (bind _bp_playerref (Variables|Ref|GetBP_PlayerRef))
  (return (>= (Math|Vector|DotProduct (Transformation|GetActorForwardVector _bp_playerref) (Math|Vector|Normalize (Pawn|Components|CharacterMovement|GetCurrentAcceleration (Variables|/Script/Engine.Character|GetCharacterMovement _bp_playerref)))) 0.707)))

(fn SetCachedWalkSpeed
  ;[0.15 0.15 0.15 0.5] 매 프레임 포즈 혹은 움직임 상태에 따라 Speed 저장
  (Utilities|FlowControl|Sequence
    (:then_0
      (LocalVariables|SetRowName (Utilities|String|ToString(Boolean) (Variables|/Game/Blueprints/Character/BP_Player.BP_Player_C|GetbIsWeaponEquipped (Variables|Ref|GetBP_PlayerRef)))))
    (:then_1
      (LocalVariables|SetRowName (Utilities|String|Append (LocalVariables|GetRowName) "_" (Utilities|String|EnumtoString (Variables|/Game/Blueprints/Character/BP_Player.BP_Player_C|GetCurrentPoseState (Variables|Ref|GetBP_PlayerRef))))))
    (:then_2
      (bind _returnvalue (Utilities|GetDataTableRow "/Game/Blueprints/Datas/DataTable/DT_WalkSpeed.DT_WalkSpeed" (Utilities|String|StringToName (LocalVariables|GetRowName)))
        (:then
          (bind _output_get (LocalVariables|SetOutRow _returnvalue))
          (Variables|Default|SetCachedSpeedData (Utilities|Select :Index (Variables|/Game/Blueprints/Character/BP_Player.BP_Player_C|GetCurrentMoveState (Variables|Ref|GetBP_PlayerRef)) :NewEnumerator0 (.walk _output_get) :NewEnumerator1 (.jog _output_get) :NewEnumerator2 (.run _output_get) :NewEnumerator3 (.aim _output_get))))))))