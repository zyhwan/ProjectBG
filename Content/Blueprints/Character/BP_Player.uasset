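; BP_Player is the player character, handling movement, look input, free look and detection of nearby world items.
; Free look unlinks yaw from the controller, moves along the saved heading, and eases back on release via a shortest-path timeline.
; Move state is resolved by priority (aim, walk, run, jog).
; Timer-driven vicinity checks use sphere and line-of-sight traces, compare results, and broadcast changed lists for UI.
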(event EventBeginPlay
  (Utilities|Time|SetTimerbyEvent (EventDispatchers|CreateEvent :!event UpdateVicinityList) 0.05 true))

(event EventTick
  (params (DeltaSeconds :type Float%20%28single-precision%29))
  (bind _returnvalue (Transformation|GetVelocity))
  (bind _returnvalue_2 (Math|Vector|VectorLengthSquared _returnvalue))
  (bind _returnvalue_3 (> _returnvalue_2 0.0))
  (if (!= (Variables|Move|GetbIsMovingNow) _returnvalue_3)
    (bind _output_get (Variables|Move|SetbIsMovingNow _returnvalue_3))
    (Default|CallOnMovementStateChange _output_get)))

(event Custom|OnFreeLookEnded
  ;[0.15 0.15 0.15 0.5] 함수로 따지면 구현부.
  (bind _alpha (Timeline|Timeline PlayFromStart)
    (:Update
      (Pawn|SetControlRotation (Pawn|GetController) (Math|Rotator|Lerp(Rotator) (Variables|FreeLook|GetFreeLookEndRotation) (Variables|FreeLook|GetFreeLookStartRotation) _alpha true)))
    (:Finished
      (Variables|Default|SetbUseControllerRotationYaw true))))

(fn ConstructionScript)

(fn InputTurn
  (params (X%20Axis :type Float%20%28double-precision%29))
  (Pawn|Input|AddControllerYawInput X%20Axis))

(fn InputLookUp
  (params (Y%20Axis :type Float%20%28double-precision%29))
  (Pawn|Input|AddControllerPitchInput Y%20Axis))

(fn Move
  (params (bIsForward :type Boolean) (Axis%20Value :type Float%20%28double-precision%29))
  (bind _busecontrollerrotationyaw (Variables|Default|GetbUseControllerRotationYaw))
  (if bIsForward
    ;[0.15 0.15 0.15 0.5] Scale Value에 따라서 몇배율로 증폭 시킬지.
    (Pawn|Input|AddMovementInput (Math|Vector|GetForwardVector (Movement|WhoDirection _busecontrollerrotationyaw)) Axis%20Value false)
    (else
      (Pawn|Input|AddMovementInput (Math|Vector|GetRightVector (Movement|WhoDirection _busecontrollerrotationyaw)) Axis%20Value false))))

(fn FreeLook
  (params (bIsPressed :type Boolean))
  (bind _returnvalue (Pawn|GetControlRotation :!class /Script/Engine.Pawn))
  (if bIsPressed
    (Variables|FreeLook|SetFreeLookStartRotation _returnvalue)
    (Variables|Default|SetbUseControllerRotationYaw false)
    (else
      (Variables|FreeLook|SetFreeLookEndRotation _returnvalue)
      (CallFunction|OnFreeLookEnded))))

(fn WhoDirection
  (params (FreeLook :type Boolean))
  (return (Math|Rotator|SelectRotator (CallFunction|GetYawOnlyRotation (Pawn|GetControlRotation self :!class /Script/Engine.Pawn)) (CallFunction|GetYawOnlyRotation (Variables|FreeLook|GetFreeLookStartRotation)) FreeLook)))

(fn UpdatePoseState
  (params (NewState :type E_PoseState%20Enum :default "NewEnumerator0"))
  (Variables|Pose|SetCurrentPoseState NewState))

(fn UpdateMoveState
  (params (NewState :type E_MoveState%20Enum :default "NewEnumerator0"))
  (Variables|Move|SetCurrentMoveState NewState))

(fn EvaluateMoveState
  (Utilities|FlowControl|Sequence
    (:then_0
      (Variables|Move|SetCurrentMoveState "NewEnumerator1"))
    (:then_1
      (if (Variables|Move|GetbIsRunPresssed)
        (Variables|Move|SetCurrentMoveState "NewEnumerator2")))
    (:then_2
      (if (Variables|Move|GetbIsWalkPressed)
        (Variables|Move|SetCurrentMoveState "NewEnumerator0")))
    (:then_3
      (if (Variables|Move|GetbIsAimpressed)
        (Variables|Move|SetCurrentMoveState "NewEnumerator3")))))

(fn SetMaxWalkSpeed
  (params (NewSpeed :type Float%20%28double-precision%29))
  (Variables|/Script/Engine.CharacterMovementComponent|SetMaxWalkSpeed (Variables|Character|GetCharacterMovement) NewSpeed))

(fn GetVicinityItems
  (bind _returnvalue (Transformation|GetActorLocation))
  (bind _returnvalue_2 (Transformation|GetActorLocation))
  ;[0.15 0.15 0.15 0.5] 오브젝트 채널을 기준으로 검색을 함.
  (bind _outhits (Collision|MultiSphereTraceForObjects _returnvalue_2 _returnvalue_2 2.2e+02 (Utilities|Array|MakeArray "ObjectTypeQuery8") false 0 "ForDuration" true "(R=1.000000,G=0.000000,B=0.000000,A=1.000000)" "(R=0.000000,G=1.000000,B=0.000000,A=1.000000)" 0.03))
  (for _array_element _outhits
    (bind _outhit (Collision|LineTraceByChannel (Math|Vector|MakeVector (.x _returnvalue) (.y _returnvalue) (+ (.z _returnvalue) 88.0)) (Transformation|GetActorLocation (.HitActor (Collision|BreakHitResult _array_element))) "TraceTypeQuery1" false 0 "ForDuration" true "(R=1.000000,G=0.000000,B=0.000000,A=1.000000)" "(R=0.000000,G=1.000000,B=0.000000,A=1.000000)" 0.03))
    (if (== (.HitActor (Collision|BreakHitResult _outhit)) (.HitActor (Collision|BreakHitResult _array_element)))
      (Utilities|Set|Add (LocalVariables|GetReturnVicinityItems) (.HitActor (Collision|BreakHitResult _array_element)))))
  (return (LocalVariables|GetReturnVicinityItems)))

(fn UpdateVicinityList
  ;[0.15 0.15 0.15 0.5] 타이머의 이전 이벤트와 현재 이벤트의 충돌 체크에서 아이템 체크의 변동사항이 있는지 체크한다. 변동 사항이 없으면 갱신하지 않음.
  (Utilities|FlowControl|Sequence
    (:then_0
      ;;[0.15 0.15 0.15 0.5] 1차 변동사항 체크, 개숫가 동일한지 체크
      (bind _output_get (LocalVariables|SetNewVicinityItems (CallFunction|GetVicinityItems)))
      (if (== (Utilities|Set|Length _output_get) (Utilities|Set|Length (LocalVariables|GetOldVicinityItems)))
        ;;[0.15 0.15 0.15 0.5] 2차 변동사항 체크, 포함된 내용이 같은지
        (bind _valuepin (Utilities|Set|ForEachLoop(Set) (LocalVariables|GetNewVicinityItems) :!label _label)
          (:then
            (if (not (Utilities|Set|Contains (LocalVariables|GetOldVicinityItems) _valuepin))
              (LocalVariables|SetbNeedUpdate true)
              (goto _label BreakPin))))
        (else
          (LocalVariables|SetbNeedUpdate true))))
    (:then_1
      ;;[0.15 0.15 0.15 0.5] UI 업데이트가 필요한지 여부
      (if (LocalVariables|GetbNeedUpdate)
        (Utilities|Set|Clear (Variables|Default|GetCurrentVicinityItems))
        (bind _valuepin_2 (Utilities|Set|ForEachLoop(Set) (LocalVariables|GetNewVicinityItems))
          (:then
            (bind _asbp_world_item_base (Utilities|Casting|CastToBP_WorldItemBase _valuepin_2))
            (Utilities|Set|Add (Variables|Default|GetCurrentVicinityItems) _asbp_world_item_base))
          (:CompletedPin
            (Default|CallOnVicinityItemsUpdated (Variables|Default|GetCurrentVicinityItems))))))))