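; Game mode that scatters random loot at BeginPlay, spawning a BP_ItemGroup at each DT_ItemGroupLocations row.
; It first caches row names and percent totals from the probability DataTables, though none for Weapon.
; Each group rolls an item count, distinct types (re-rolling duplicates) and an ID per type, then spawns BP_TestItem at the group's random transforms.
; Rolls are cumulative-percent weighted picks with early return.
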(event EventBeginPlay
  (CallFunction|GenerateItems))

(fn ConstructionScript)

(fn GenerateItems
  ;[0.15 0.15 0.15 0.5] 아이템에 대한 데이터 테이블 가져오기
  (|CollapseGraph
    (:Out%20Execute
      ;[0.15 0.15 0.15 0.5] 위치를 지정한 아이템 그룹을 스폰
      (bind _outrownames (DataTable|GetDataTableRowNames "/Game/Blueprints/Datas/DataTable/ITemGeneration/DT_ItemGroupLocations.DT_ItemGroupLocations"))
      (for _array_element _outrownames
        (bind _returnvalue (Utilities|GetDataTableRow "/Game/Blueprints/Datas/DataTable/ITemGeneration/DT_ItemGroupLocations.DT_ItemGroupLocations" _array_element)
          (:then
            (bind _returnvalue_2 (Game|SpawnActorfromClass "/Game/Blueprints/Items/BP_ItemGroup.BP_ItemGroup_C" (Math|Transform|MakeTransform (.location _returnvalue) "0, 0, 0" "1.000000,1.000000,1.000000") "Undefined" "MultiplyWithRoot" 0 0))
            (LocalVariables|SetItemGroupRef _returnvalue_2)
            (Utilities|Array|Clear (LocalVariables|GetItemTypeArray))
            ;[0.15 0.15 0.15 0.5] 랜덤한 아이템 개수 정하기
            (bind _number (CallFunction|RandomItemNumber (LocalVariables|GetNumberProbabilityInfo)))
            (LocalVariables|SetSpawnTransforms (Default|GetRandomTransform (LocalVariables|GetItemGroupRef) _number))
            (for _index (range 1 _number)
              ;[0.15 0.15 0.15 0.5] 랜덤한 아이템 타입 뽑기
              (bind _itemtype (CallFunction|RandomItemType (LocalVariables|GetItemTypeProbabilityInfo) :!label _label))
              ;[0.15 0.15 0.15 0.5] 중복 방지
              (if (== (Utilities|Array|FindItem (LocalVariables|GetItemTypeArray) _itemtype) -1)
                (Utilities|Array|Add (LocalVariables|GetItemTypeArray) _itemtype)
                (else
                  (goto _label))))
            (for _array_element_2 (LocalVariables|GetItemTypeArray)
              (bind _spawnitem (CallFunction|RandomItemID (LocalVariables|GetItemIdProbabilityInfos) _array_element_2))
              (Utilities|Array|Add (LocalVariables|GetSpawnItemArr) _spawnitem))
            (for (_array_element_3 _array_index) (LocalVariables|GetSpawnItemArr)
              (LocalVariables|SetItemType (.itemtype _array_element_3))
              (LocalVariables|SetSpawnId (.id _array_element_3))
              (Game|SpawnActorfromClass "/Game/Blueprints/BP_TestItem.BP_TestItem_C" (Utilities|Array|Get(acopy) (LocalVariables|GetSpawnTransforms) _array_index) "Undefined" "MultiplyWithRoot" 0 0))
            (Utilities|Array|Clear (LocalVariables|GetSpawnItemArr))))))))

(fn RandomItemNumber
  (params (NumberProbability :type ST%20Probability%20Info%20Structure))
  ;[0.15 0.15 0.15 0.5] 메모리 낭비가 적고 반복횟수를 낮춤.
  (LocalVariables|SetRandomValue (Math|Random|RandomIntegerinRange 1 (.totalpercent NumberProbability)))
  (for _array_element (.rownames NumberProbability)
    (bind _returnvalue (Utilities|GetDataTableRow "/Game/Blueprints/Datas/DataTable/ITemGeneration/DT_NumberProbabilitys.DT_NumberProbabilitys" _array_element)
      (:then
        (bind _output_get (LocalVariables|SetSumPercent (+ (LocalVariables|GetSumPercent) (.percent _returnvalue))))
        ;;[0.15 0.15 0.15 0.5] 얼리 리턴
        (if (>= _output_get (LocalVariables|GetRandomValue))
          (return (.number _returnvalue)))))))

(fn RandomItemType
  (params (ItemTypeProbabilityInfo :type ST%20Probability%20Info%20Structure))
  (LocalVariables|SetRandomValue (Math|Random|RandomIntegerinRange 1 (.totalpercent ItemTypeProbabilityInfo)))
  (for _array_element (.rownames ItemTypeProbabilityInfo)
    (bind _returnvalue (Utilities|GetDataTableRow "/Game/Blueprints/Datas/DataTable/ITemGeneration/DT_ItemTypeProbabilitys.DT_ItemTypeProbabilitys" _array_element)
      (:then
        (bind _output_get (LocalVariables|SetSumPercent (+ (.percent _returnvalue) (LocalVariables|GetSumPercent))))
        (if (>= _output_get (LocalVariables|GetRandomValue))
          (return (.itemtype _returnvalue)))))))

(fn RandomItemID
  (params (ItemIDProbabilityInfos :type Map%20of%20E_ItemType%20Enums%20to%20Structs :default "NewEnumerator0") (ItemType :type E_ItemType%20Enum :default "NewEnumerator0"))
  (bind _value (Utilities|Map|Find ItemIDProbabilityInfos ItemType))
  (bind (_totalpercent _rownames) (Utilities|Struct|BreakST_ProbabilityInfo _value))
  (LocalVariables|SetRandomValue (Math|Random|RandomIntegerinRange 1 _totalpercent))
  (for _array_element _rownames
    (bind _returnvalue (Utilities|GetDataTableRow (Utilities|Select :Index ItemType :NewEnumerator0 "/Game/Blueprints/Datas/DataTable/ITemGeneration/DT_WeaponProbabilitys.DT_WeaponProbabilitys" :NewEnumerator1 "/Game/Blueprints/Datas/DataTable/ITemGeneration/DT_WeaponAccProbabiliys.DT_WeaponAccProbabiliys" :NewEnumerator2 "/Game/Blueprints/Datas/DataTable/ITemGeneration/DT_AmmoProbabilitys.DT_AmmoProbabilitys" :NewEnumerator3 "/Game/Blueprints/Datas/DataTable/ITemGeneration/DT_HealthProbabiliys.DT_HealthProbabiliys" :NewEnumerator4 "/Game/Blueprints/Datas/DataTable/ITemGeneration/DT_BoostProbabiliys.DT_BoostProbabiliys" :NewEnumerator5 "/Game/Blueprints/Datas/DataTable/ITemGeneration/DT_HelmetProbabilitys.DT_HelmetProbabilitys" :NewEnumerator6 "/Game/Blueprints/Datas/DataTable/ITemGeneration/DT_VestProbabilitys.DT_VestProbabilitys" :NewEnumerator7 "/Game/Blueprints/Datas/DataTable/ITemGeneration/DT_BackpackProbabilitys.DT_BackpackProbabilitys") _array_element)
      (:then
        (bind _output_get (LocalVariables|SetSumPercent (+ (LocalVariables|GetSumPercent) (Utilities|Struct|BreakST_ItemProbability _returnvalue))))
        (if (>= _output_get (LocalVariables|GetRandomValue))
          (return (Utilities|Struct|MakeST_SpawnItem ItemType _array_element)))))))