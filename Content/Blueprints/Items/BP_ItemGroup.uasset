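; BP_ItemGroup is an item group actor that generates random positions scattered around its own location.
; GetRandomTransform builds a requested number of transforms, offsetting each from the actor by a random unit vector scaled to a random 100–200 cm length.
; Only X and Y of the offset are kept, so points share the actor's height and can land closer than 100 cm.
; Rotation and scale stay at defaults, and the construction script is empty.
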(fn ConstructionScript)

(fn GetRandomTransform
  (params (Number :type Integer))
  (bind _returnvalue (Math|Random|RandomUnitVector))
  (bind _returnvalue_2 (Math|Random|RandomFloatinRange 1e+02 2e+02))
  (bind _returnvalue_3 (* _returnvalue _returnvalue_2))
  ;[0.15 0.15 0.15 0.5] 아이템 그룹 100~200cm 이내 랜덤한 위치 배열 생성
  (for _index (range 1 Number)
    (Utilities|Array|Add (LocalVariables|GetReturnTransforms) (Math|Transform|MakeTransform (+ (Transformation|GetActorLocation) (Math|Vector|MakeVector (.x _returnvalue_3) (.y _returnvalue_3) 0.0)))))
  (return (LocalVariables|GetReturnTransforms)))